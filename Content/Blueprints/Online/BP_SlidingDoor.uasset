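; Door Blueprint that slides its Cube mesh along Z between closed and open positions.
; OpenDoor toggles the Open flag and plays or reverses the OpeningDoor timeline, whose Zpos scales MaxLocation as an offset from the location cached at BeginPlay.
; The Sphere trigger registers this door in BP_FirstPersonCharacter's Door variable on begin overlap.
; End overlap assigns the same reference instead of clearing it.
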(event OnComponentBeginOverlap(Sphere)
  (params (OverlappedComponent :type Primitive%20Component%20Object%20Reference) (OtherActor :type Actor%20Object%20Reference) (OtherComp :type Primitive%20Component%20Object%20Reference) (OtherBodyIndex :type Integer) (bFromSweep :type Boolean) (SweepResult :type Hit%20Result%20Structure%20%28by%20ref%29))
  (bind _asbp_first_person_character (Utilities|Casting|CastToBP_FirstPersonCharacter OtherActor))
  (Variables|/Game/Blueprints/Pawns/BP_FirstPersonCharacter.BP_FirstPersonCharacter_C|SetDoor _asbp_first_person_character self))

(event OnComponentEndOverlap(Sphere)
  (params (OverlappedComponent :type Primitive%20Component%20Object%20Reference) (OtherActor :type Actor%20Object%20Reference) (OtherComp :type Primitive%20Component%20Object%20Reference) (OtherBodyIndex :type Integer))
  (bind _asbp_first_person_character (Utilities|Casting|CastToBP_FirstPersonCharacter OtherActor))
  (Variables|/Game/Blueprints/Pawns/BP_FirstPersonCharacter.BP_FirstPersonCharacter_C|SetDoor _asbp_first_person_character self))

(event Custom|OpenDoor
  (if (Variables|Default|GetOpen)
    (Variables|Default|SetOpen false)
    (bind _zpos (Timeline|Opening%20Door Reverse)
      (:Update
        (Transformation|SetRelativeLocation (Variables|Default|GetCube) (+ (Math|Vector|MakeVector 0.0 0.0 (* (Variables|Default|GetMaxLocation) _zpos)) (Variables|Default|GetStartLocation)) false false)))
    (else
      (Variables|Default|SetOpen true)
      (Timeline|Opening%20Door Play))))

(event EventBeginPlay
  (Variables|Default|SetStartLocation (Variables|/Script/Engine.SceneComponent|GetRelativeLocation (Variables|Default|GetCube))))

(fn ConstructionScript)