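; Game State Blueprint that keeps a kill and death scoreboard, with one entry per player pseudo in a Scores array.
; AddPlayer appends a zeroed entry only when a linear Find shows the pseudo is new, then announces the score update.
; Srv_AddKill announces the kill, increments the killer's kills and the victim's deaths, then announces the update.
; Multi_ events relay both notifications through event dispatchers for listeners.
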(event Custom|Srv_AddKill
  (params (Killer :type String) (Killed :type String))
  (CallFunction|MultionNewKill Killer Killed)
  (CallFunction|AugmentScore Killer true)
  (CallFunction|AugmentScore Killed false)
  (CallFunction|MultionScoreUpdate))

(event Custom|AddPlayer
  (params (Pseudo :type String))
  (bind _added (CallFunction|Add (Utilities|Struct|MakeSScoreInfos Pseudo)))
  (if _added
    (CallFunction|MultionScoreUpdate)))

(event Custom|Multi_OnNewKill
  (params (Killer :type String) (Killed :type String))
  (Default|CallOnNewKil Killer Killed))

(event Custom|Multi_OnScoreUpdate
  (Default|CallOnScoreUpdate))

(fn ConstructionScript)

(fn Find
  (params (Pseudo :type String))
  (bind (_array_element _array_index) (Utilities|Array|ForEachLoopwithBreak (Variables|Default|GetScores) :!label _label)
    (:LoopBody
      (if (Utilities|Enum|Equal(Enum) (Utilities|Struct|BreakSScoreInfos _array_element) Pseudo)
        (LocalVariables|SetFoundIndex _array_index)
        (goto _label Break)))
    (:Completed
      (return (LocalVariables|GetFoundIndex) (!= (LocalVariables|GetFoundIndex) -1)))))

(fn Add
  (params (Infos :type S%20Score%20Infos%20Structure))
  (if (.Found (CallFunction|Find (Utilities|Struct|BreakSScoreInfos Infos)))
    (return -1 false)
    (else
      (bind _returnvalue (Utilities|Array|Add (Variables|Default|GetScores) Infos))
      (return _returnvalue true))))

(fn AugmentScore
  (params (Pseudo :type String) (Kill :type Boolean))
  (bind (_index _found) (CallFunction|Find Pseudo))
  (bind _scores (Variables|Default|GetScores))
  (bind _output (Utilities|Array|Get(acopy) _scores _index))
  (bind (_kills _deaths) (Utilities|Struct|BreakSScoreInfos _output))
  (if _found
    (if Kill
      (Math|Integer|IncrementInt _kills)
      (else
        (Math|Integer|IncrementInt _deaths)))))