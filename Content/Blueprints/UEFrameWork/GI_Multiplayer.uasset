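; Multiplayer game instance that persists the client's player name (Pseudo) and the server's kill/death scores through SaveGame slots.
; Client loading restores the saved Pseudo only when the current one is empty.
; Server saving reloads stored scores, merges in the GameState's scores, then writes asynchronously.
; MergeScores matches entries by Pseudo, replacing saved ones with current-game values rather than summing, and appends new players.
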(event Custom|ClientSave
  (bind _returnvalue (SaveGame|CreateSaveGameObject "/Game/Blueprints/Structs/SG_ClientSave.SG_ClientSave_C"))
  (Variables|/Game/Blueprints/Structs/SG_ClientSave.SG_ClientSave_C|SetPseudo _returnvalue (Variables|Default|GetPseudo))
  (SaveGame|SaveGametoSlot _returnvalue "ClientInfos"))

(event Custom|LoadClient
  (bind _returnvalue (SaveGame|LoadGamefromSlot "ClientInfos"))
  (Utilities|IsValid _returnvalue
    (:Is%20Valid
      (bind _assg_client_save (Utilities|Casting|CastToSG_ClientSave _returnvalue))
      (if (Utilities|Enum|Equal(Enum) (Variables|Default|GetPseudo) "")
        (Variables|Default|SetPseudo (Variables|/Game/Blueprints/Structs/SG_ClientSave.SG_ClientSave_C|GetPseudo _assg_client_save))))))

(event Custom|LoadServer
  (bind _returnvalue (SaveGame|LoadGamefromSlot "ServerInfos"))
  (Utilities|IsValid _returnvalue
    (:Is%20Valid
      (bind _assg_server_save (Utilities|Casting|CastToSG_ServerSave _returnvalue))
      (bind _output_get (Variables|Default|SetSavedScores (Variables|/Game/Blueprints/Structs/SG_ServerSave.SG_ServerSave_C|GetScores _assg_server_save))))))

(event Custom|SaveServer
  (CallFunction|LoadServer)
  (bind _returnvalue (SaveGame|CreateSaveGameObject "/Game/Blueprints/Structs/SG_ServerSave.SG_ServerSave_C"))
  (bind _mergedarray (CallFunction|MergeScores (Variables|Default|GetSavedScores) (Variables|/Game/Blueprints/UEFrameWork/BP_GameState.BP_GameState_C|GetScores (.AsBP%20Game%20State (Utilities|Casting|CastToBP_GameState (Game|GetGameState))))))
  (Variables|/Game/Blueprints/Structs/SG_ServerSave.SG_ServerSave_C|SetScores _returnvalue _mergedarray)
  (|AsyncSaveGametoSlot _returnvalue "ServerInfos"))

(fn MergeScores
  (params (SaveArray :type Array%20of%20S%20Score%20Infos%20Structures) (GameScores :type Array%20of%20S%20Score%20Infos%20Structures))
  (bind _outarray (LocalVariables|GetOutArray))
  (Utilities|Array|Clear (LocalVariables|GetOutArray))
  (LocalVariables|SetScoresToTest GameScores)
  (for _array_element SaveArray
    (if (.Found (CallFunction|Find (LocalVariables|GetScoresToTest) (Utilities|Struct|BreakSScoreInfos _array_element)))
      (Utilities|Array|Add _outarray (Utilities|Array|Get(acopy) (LocalVariables|GetScoresToTest) (.Index (CallFunction|Find (LocalVariables|GetScoresToTest) (Utilities|Struct|BreakSScoreInfos _array_element)))))
      (Utilities|Array|RemoveItem (LocalVariables|GetScoresToTest) (Utilities|Array|Get(acopy) (LocalVariables|GetScoresToTest) (.Index (CallFunction|Find (LocalVariables|GetScoresToTest) (Utilities|Struct|BreakSScoreInfos _array_element)))))
      (else
        (Utilities|Array|Add _outarray _array_element))))
  (Utilities|Array|AppendArray (LocalVariables|GetOutArray) (LocalVariables|GetScoresToTest))
  (return (LocalVariables|GetOutArray)))

(fn Find
  (params (Array :type Array%20of%20S%20Score%20Infos%20Structures) (Pseudo :type String))
  (bind (_array_element _array_index) (Utilities|Array|ForEachLoopwithBreak Array :!label _label)
    (:LoopBody
      (if (Utilities|Enum|Equal(Enum) (Utilities|Struct|BreakSScoreInfos _array_element) Pseudo)
        (LocalVariables|SetFoundIndex _array_index)
        (goto _label Break)))
    (:Completed
      (return (LocalVariables|GetFoundIndex) (!= (LocalVariables|GetFoundIndex) -1)))))

(fn PrintDebug
  (params (Array :type Array%20of%20S%20Score%20Infos%20Structures))
  (for _array_element Array
    (Development|PrintString (Utilities|String|Append (.Pseudo (Utilities|Struct|BreakSScoreInfos _array_element)) (Utilities|String|ToString(Integer) (.Kills (Utilities|Struct|BreakSScoreInfos _array_element))) (Utilities|String|ToString(Integer) (.Deaths (Utilities|Struct|BreakSScoreInfos _array_element)))))))