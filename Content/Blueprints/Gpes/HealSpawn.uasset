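; A healing pickup pad that refills after use.
; When a BP_MeleeChara overlaps its capsule, the pad passes itself to that character's HealPad function.
; HealByPlayer hides the mesh and disables capsule collision, then restores both as query-only after the RefillTime delay.
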(event OnComponentBeginOverlap(Capsule)
  (params (OverlappedComponent :type Primitive%20Component%20Object%20Reference) (OtherActor :type Actor%20Object%20Reference) (OtherComp :type Primitive%20Component%20Object%20Reference) (OtherBodyIndex :type Integer) (bFromSweep :type Boolean) (SweepResult :type Hit%20Result%20Structure%20%28by%20ref%29))
  (bind _asbp_melee_chara (Utilities|Casting|CastToBP_MeleeChara OtherActor))
  (Default|HealPad _asbp_melee_chara self))

(event Custom|HealByPlayer
  (Rendering|SetVisibility (Variables|Default|GetStaticMesh) false true)
  (Collision|SetCollisionEnabled (Variables|Default|GetCapsule) "NoCollision")
  (Utilities|FlowControl|Delay (Variables|Default|GetRefillTime))
  (Rendering|SetVisibility (Variables|Default|GetStaticMesh) true true)
  (Collision|SetCollisionEnabled (Variables|Default|GetCapsule) "QueryOnly"))

(fn ConstructionScript)