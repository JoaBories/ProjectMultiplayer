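; BP_HealSpawn is a spawn point that keeps a BP_Heal actor replenished in the level.
; On BeginPlay, the authority starts a looping timer at the RefillTime interval.
; Each tick of that timer spawns a new heal at the SpawnPoint component only if the stored one is no longer valid, so one exists at a time.
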(event Custom|TrySpawn
  (Utilities|IsValid (Variables|Default|GetHeal)
    (:Is%20Not%20Valid
      (bind _returnvalue (Game|SpawnActorfromClass "/Game/Blueprints/Gpes/BP_Heal.BP_Heal_C" (Math|Transform|MakeTransform (Transformation|GetWorldLocation (Variables|Default|GetSpawnPoint)) "0, 0, 0" "1.000000,1.000000,1.000000") "AlwaysSpawn" "MultiplyWithRoot" 0 0))
      (Variables|Default|SetHeal _returnvalue))))

(event EventBeginPlay
  (if (Ability|HasAuthority)
    (Utilities|Time|SetTimerbyEvent (delegate Custom|TrySpawn) (Variables|Default|GetRefillTime) true)))

(fn ConstructionScript)