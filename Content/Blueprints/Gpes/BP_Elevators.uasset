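; BP_Elevators is an elevator platform that makes a round trip between StartPos and EndPos when triggered.
; A BP_MeleeChara entering the Box calls its own SrvStartElevator with this actor, while StartUp begins the ascent.
; Tick moves the Cube along the normalized start-to-end direction at Speed, using GoingUp and GoingDown flags.
; It waits briefly at EndPos, then returns and snaps to StartPos.
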(event OnComponentBeginOverlap(Box)
  (params (OverlappedComponent :type Primitive%20Component%20Object%20Reference) (OtherActor :type Actor%20Object%20Reference) (OtherComp :type Primitive%20Component%20Object%20Reference) (OtherBodyIndex :type Integer) (bFromSweep :type Boolean) (SweepResult :type Hit%20Result%20Structure%20%28by%20ref%29))
  (bind _asbp_melee_chara (Utilities|Casting|CastToBP_MeleeChara OtherActor))
  (Default|SrvStartElevator _asbp_melee_chara self))

(event Custom|StartUp
  (Variables|Default|SetGoingUp true))

(event EventTick
  (params (DeltaSeconds :type Float%20%28single-precision%29))
  (bind _cube (Variables|Default|GetCube))
  (bind _cube_2 (Variables|Default|GetCube))
  (if (Variables|Default|GetGoingUp)
    (Transformation|SetWorldLocation _cube_2 (CallFunction|GetNewLocation DeltaSeconds true) false false)
    (if (Utilities|Operators|EqualEqual (Transformation|GetWorldLocation (Variables|Default|GetEndPos)) (Transformation|GetWorldLocation _cube_2) 1.0)
      (Variables|Default|SetGoingUp false)
      (Utilities|FlowControl|Delay 2.0)
      (Variables|Default|SetGoingDown true))
    (elif (Variables|Default|GetGoingDown)
      (Transformation|SetWorldLocation _cube (CallFunction|GetNewLocation DeltaSeconds false) false false)
      (if (Utilities|Operators|EqualEqual (Transformation|GetWorldLocation (Variables|Default|GetStartPos)) (Transformation|GetWorldLocation _cube) 1.0)
        (Variables|Default|SetGoingDown false)
        (Transformation|SetWorldLocation (Variables|Default|GetCube) (Transformation|GetWorldLocation (Variables|Default|GetStartPos)) false false)))))

(event EventBeginPlay
  (Variables|Default|SetDirection (Math|Vector|Normalize (- (Transformation|GetWorldLocation (Variables|Default|GetEndPos)) (Transformation|GetWorldLocation (Variables|Default|GetStartPos))))))

(fn ConstructionScript)

(fn GetNewLocation
  (params (DeltaTime :type Float%20%28single-precision%29) (Up :type Boolean))
  (bind _direction (Variables|Default|GetDirection))
  (return (+ (Transformation|GetWorldLocation (Variables|Default|GetCube)) (* (Math|Vector|SelectVector _direction (Math|Vector|NegateVector _direction) Up) DeltaTime (Variables|Default|GetSpeed)))))