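; BP_SlidingDoor is an interactable door that slides its Cube mesh along the Z axis to open and close.
; Interact toggles the Open state, playing or reversing a timeline that offsets the Cube from its starting relative location by up to MaxLocation.
; A DoOnce reset after a short delay debounces repeated interactions.
; IsLocal returns false and ShowWidget returns the actor's location.
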(event EventBeginPlay
  (Variables|Default|SetStartLocation (Variables|/Script/Engine.SceneComponent|GetRelativeLocation (Variables|Default|GetCube))))

(event EventInteract
  (Utilities|FlowControl|DoOnce false :!label _label
    (:Completed
      (Utilities|FlowControl|Sequence
        (:then_0
          (if (not (Variables|Default|GetOpen))
            (Variables|Default|SetOpen true)
            (bind _zpos (Timeline|Opening%20Door Play)
              (:Update
                (Transformation|SetRelativeLocation (Variables|Default|GetCube) (+ (Math|Vector|MakeVector 0.0 0.0 (* (Variables|Default|GetMaxLocation) _zpos)) (Variables|Default|GetStartLocation)) false false)))
            (else
              (Variables|Default|SetOpen false)
              (Timeline|Opening%20Door Reverse))))
        (:then_1
          (Utilities|FlowControl|Delay 0.2)
          (goto _label Reset))))))

(fn ConstructionScript)

(fn IsLocal
  (return false))

(fn ShowWidget
  (return (Transformation|GetActorLocation)))