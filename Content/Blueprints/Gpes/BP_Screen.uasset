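; BP_Screen is an actor that shows the current best score on a WBP_BestScore widget component.
; On BeginPlay it waits tick by tick until BP_GameState is available, then binds to its score update event and caches the widget.
; Each update scans the game state's scores for the entry with the most kills and passes it to the widget.
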(event Custom|OnScoreUpdate
  (bind _gamestate (Variables|Default|GetGameState))
  (bind _scores (Variables|/Game/Blueprints/UEFrameWork/BP_GameState.BP_GameState_C|GetScores _gamestate))
  (Variables|Default|SetBestScore (Utilities|Array|Get(acopy) _scores))
  (for _array_element _scores
    (if (> (Utilities|Struct|BreakSScoreInfos _array_element) (.kills (Variables|Default|GetBestScore)))
      (Variables|Default|SetBestScore _array_element)))
  (Default|UpdateInfos (Variables|Default|GetBestScoreWidget) (Variables|Default|GetBestScore)))

(event EventBeginPlay
  (bind _asbp_game_state (Utilities|Casting|CastToBP_GameState (Game|GetGameState) :!label _label)
    (:then
      (bind _output_get (Variables|Default|SetGameState _asbp_game_state))
      (EventDispatchers|BindEventtoOnScoreUpdate _output_get (delegate Custom|OnScoreUpdate))
      (bind _aswbp_best_score (Utilities|Casting|CastToWBP_BestScore (UserInterface|GetWidget (Variables|Default|GetWidget))))
      (Variables|Default|SetBestScoreWidget _aswbp_best_score))
    (:CastFailed
      (Utilities|FlowControl|DelayUntilNextTick)
      (goto _label))))

(fn ConstructionScript)