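; AC_Interact is an actor component on BP_MeleeChara that lets the player interact with nearby actors.
; On the locally controlled owner it creates a screen-space widget component showing a hidden WBP_Interact prompt.
; Zone enter and exit events track the current interactable, moving and attaching the prompt to it or hiding it.
; Input calls the interactable's interface locally or routes it through the character's SrvInteract, depending on IsLocalMessage.
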(event Custom|ExitInteractZone
  (params (Actor :type Actor%20Object%20Reference))
  (if (== Actor (Variables|Default|GetCurrentInteraction))
    (Variables|Default|SetCurrentInteraction 0)
    (Widget|SetRenderOpacity (Variables|Default|GetWidget) 0.0)))

(event Custom|EnterInteractZone
  (params (Actor :type Actor%20Object%20Reference))
  (bind _widgetcomponent (Variables|Default|GetWidgetComponent))
  (Variables|Default|SetCurrentInteraction Actor)
  (Widget|SetRenderOpacity (Variables|Default|GetWidget) 1.0)
  (bind _getinteractpos (Class|BPIInteract|ShowWidget(Message) (Variables|Default|GetCurrentInteraction)))
  (Transformation|SetWorldLocation _widgetcomponent _getinteractpos false false)
  (Transformation|AttachComponentToComponent _widgetcomponent (Variables|/Script/Engine.Actor|GetRootComponent (Variables|Default|GetCurrentInteraction)) "None" "KeepWorld" "KeepWorld" "KeepWorld" true))

(event Custom|Input
  (bind _currentinteraction (Variables|Default|GetCurrentInteraction))
  (Utilities|IsValid _currentinteraction
    (:Is%20Valid
      (bind _local (Class|BPIInteract|IsLocal(Message) _currentinteraction))
      (if _local
        (Class|BPIInteract|Interact(Message) _currentinteraction)
        (else
          (Default|SrvInteract (Variables|Default|GetOwner) _currentinteraction))))))

(event EventBeginPlay
  (bind _output_get (Variables|Default|SetOwner (.AsBP%20Melee%20Chara (Utilities|Casting|CastToBP_MeleeChara (Components|GetOwner)))))
  (if (Pawn|IsLocallyControlled _output_get)
    (bind _returnvalue (Game|AddComponentbyClass (Components|GetOwner) "/Script/UMG.WidgetComponent" false))
    (bind _output_get_2 (Variables|Default|SetWidgetComponent _returnvalue))
    (Class|WidgetComponent|SetWidgetSpace _output_get_2 "Screen")
    (Class|WidgetComponent|SetDrawSize _output_get_2 "(X=200.000000,Y=80.000000)")
    (bind _returnvalue_2 (UserInterface|CreateWidget "/Game/Blueprints/Menus/WBP_Interact.WBP_Interact_C"))
    (bind _output_get_3 (Variables|Default|SetWidget _returnvalue_2))
    (UserInterface|SetWidget _output_get_2 _output_get_3)
    (Widget|SetRenderOpacity _output_get_3 0.0)))